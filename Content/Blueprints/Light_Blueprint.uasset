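; Interactable light actor that toggles its point light on and off.
; LightInteract first prints a debug message shared with the plain Interact event, then compares the PointLight intensity to the LightOff variable.
; A match sets the light to a fixed bright intensity, and any other value sets it to zero.
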(event EventBeginPlay)

(event Collision|EventActorBeginOverlap
  (params (OtherActor :type Actor%20Object%20Reference)))

(event EventTick
  (params (DeltaSeconds :type Float%20%28single-precision%29)))

(event EventInteract
  (Development|PrintString "I am sphere" true true "(R=0.941667,G=1.000000,B=1.000000,A=1.000000)"))

(event EventLightInteract
  (Utilities|FlowControl|Sequence
    (:then_0
      (Development|PrintString "I am sphere" true true "(R=0.941667,G=1.000000,B=1.000000,A=1.000000)"))
    (:then_1
      (if (== (Variables|/Script/Engine.LightComponentBase|GetIntensity (Variables|Default|GetPointLight)) (Variables|Default|GetLight%20Off))
        (Rendering|Components|Light|SetIntensity (Variables|Default|GetPointLight) 5e+03)
        (else
          (Rendering|Components|Light|SetIntensity (Variables|Default|GetPointLight) 0.0))))))

(fn ConstructionScript)