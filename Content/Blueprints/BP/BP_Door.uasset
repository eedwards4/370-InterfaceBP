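; BP_Door is a door actor that slides open and closed each time its MoveDoor event is called.
; MoveDoor prints a debug string, then plays or reverses the DoorDiver timeline based on the HasPlayed flag.
; The timeline lerps the Door's relative location between DoorStart and DoorEnd, and flips HasPlayed only when finished.
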(event EventBeginPlay)

(event Collision|EventActorBeginOverlap
  (params (OtherActor :type Actor%20Object%20Reference)))

(event EventTick
  (params (DeltaSeconds :type Float%20%28single-precision%29)))

(event EventMoveDoor
  (Development|PrintString "Open Da Door")
  (if (Variables|Default|GetHasPlayed)
    (bind _driver (Timeline|Door%20Diver Reverse)
      (:Update
        (Transformation|SetRelativeLocation (Variables|Default|GetDoor) (Math|Vector|Lerp(Vector) (Variables|DoorSetup|GetDoor_Start) (Variables|DoorSetup|GetDoor_End) _driver) false false))
      (:Finished
        (if (Variables|Default|GetHasPlayed)
          (Variables|Default|SetHasPlayed false)
          (else
            (Variables|Default|SetHasPlayed true)))))
    (else
      (Timeline|Door%20Diver Play))))

(fn ConstructionScript)