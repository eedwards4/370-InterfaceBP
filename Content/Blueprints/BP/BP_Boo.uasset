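; BP_Boo is a ghost enemy that creeps toward the player only while it has not been recently rendered.
; Each Tick, unseen Boos turn and interpolate toward the pawn, while a timeline, reversed when seen, drives material opacity.
; A sphere overlap with BP_Character marks it Dead, freezes every Boo and shows the lose UI.
; Frozen Boos skip all movement and checks and have zero opacity.
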(event EventBeginPlay)

(event Collision|EventActorBeginOverlap
  (params (OtherActor :type Actor%20Object%20Reference)))

(event EventTick
  (params (DeltaSeconds :type Float%20%28single-precision%29))
  (bind _returnvalue (Game|Player|GetPlayerPawn 0))
  (bind _sphere (Variables|Default|GetSphere))
  (bind _overlappingactors (Collision|GetOverlappingActors _sphere "/Game/Blueprints/BP/BP_Character.BP_Character_C" :!class /Script/Engine.PrimitiveComponent))
  (if (Variables|Default|GetFrozen)
    (Rendering|Material|SetScalarParameterValueonMaterials (Variables|Default|GetStaticMesh) "Opacity" 0.0)
    (else
      (Utilities|FlowControl|Sequence
        (:then_0
          (if (Class|Actor|WasRecentlyRendered 0.2)
            (bind _newtrack_0 (Timeline|Timeline_0 Reverse)
              (:Update
                (Rendering|Material|SetScalarParameterValueonMaterials (Variables|Default|GetStaticMesh) "Opacity" _newtrack_0)))
            (else
              (Utilities|FlowControl|Sequence
                (:then_0
                  (Timeline|Timeline_0 Play))
                (:then_1
                  (Transformation|SetActorRotation (Math|Rotator|FindLookatRotation (Transformation|GetActorLocation) (Transformation|GetActorLocation (Game|Player|GetPlayerPawn 0))))
                  (Transformation|SetActorLocation (Math|Interpolation|VInterpTo (Transformation|GetActorLocation) (+ (Transformation|GetActorLocation _returnvalue) (Transformation|GetActorForwardVector _returnvalue)) DeltaSeconds 0.25) false false))))))
        (:then_1
          (if (> (Utilities|Array|Length _overlappingactors) 0)
            (for _array_element _overlappingactors
              (bind _asbp_character (Utilities|Casting|CastToBP_Character _array_element))
              (Variables|/Game/Blueprints/BP/BP_Character.BP_Character_C|SetDead _asbp_character true))
            (Utilities|FlowControl|Sequence
              (:then_0
                (bind _outactors (Actor|GetAllActorsOfClass "BP_Boo_C"))
                (for _array_element_2 _outactors
                  (Variables|BP_Boo_C|SetFrozen _array_element_2 true)))
              (:then_1
                (bind _returnvalue_2 (Actor|GetActorOfClass "/Game/Blueprints/BP/BP_Character.BP_Character_C"))
                (Widget|SetVisibility (Variables|/Game/Blueprints/BP/BP_Character.BP_Character_C|GetLoseCon _returnvalue_2) "Visible")))))))))

(fn ConstructionScript)