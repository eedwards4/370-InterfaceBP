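; Player character for a first-person game with mouse look, gaze-based interaction and point-to-teleport movement.
; Each tick it line-traces from the camera and notifies gazed interactables; right click uses that hit to move doors, switch lights, start the game through an activator, or otherwise teleport there unless dead.
; BeginPlay creates the timer HUD and hidden start, win and lose widgets, while a Delay on Tick counts minutes and seconds during play.
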(event Custom|GazeCheck
  (bind _camera (Variables|Default|GetCamera))
  (bind _returnvalue (Transformation|GetWorldLocation _camera))
  ;[1 1 1] Gaze check
  (bind _outhit (Collision|LineTraceByChannel _returnvalue (+ _returnvalue (* (Math|Vector|GetForwardVector _camera) 2000)) "TraceTypeQuery1" false 0 "ForOneFrame"))
  (Utilities|FlowControl|Sequence
    (:then_0
      (if (Utilities|DoesObjectImplementInterface (.HitActor (Collision|BreakHitResult _outhit)) "/Game/Blueprints/Interface/BP_Interact_Interface.BP_Interact_Interface_C")
        (Class|BPInteractInterface|Interact(Message) (.HitActor (Collision|BreakHitResult _outhit)))))))

(event EventBeginPlay
  ;[1 1 1] Setup
  (Utilities|FlowControl|Sequence
    (:then_0
      (bind _returnvalue (UserInterface|CreateWidget "/Game/Blueprints/HUD/HUD_Timer.HUD_Timer_C"))
      (UserInterface|Viewport|AddtoViewport _returnvalue 0))
    (:then_1
      (bind _returnvalue_2 (UserInterface|CreateWidget "/Game/Blueprints/HUD/HUD_GameStart.HUD_GameStart_C"))
      (bind _output_get (Variables|Default|SetGameStart _returnvalue_2))
      (UserInterface|Viewport|AddtoViewport _output_get 0)
      (Widget|SetVisibility _output_get "Hidden"))
    (:then_2
      (bind _returnvalue_3 (UserInterface|CreateWidget "/Game/Blueprints/HUD/HUD_WinCon.HUD_WinCon_C"))
      (bind _output_get_2 (Variables|Default|SetWinCon _returnvalue_3))
      (UserInterface|Viewport|AddtoViewport _output_get_2 0)
      (Widget|SetVisibility _output_get_2 "Hidden"))
    (:then_3
      (bind _returnvalue_4 (UserInterface|CreateWidget "/Game/Blueprints/HUD/HUD_LoseCon.HUD_LoseCon_C"))
      (bind _output_get_3 (Variables|Default|SetLoseCon _returnvalue_4))
      (UserInterface|Viewport|AddtoViewport _output_get_3 0)
      (Widget|SetVisibility _output_get_3 "Hidden"))))

(event EventTick
  (params (DeltaSeconds :type Float%20%28single-precision%29))
  ;[1 1 1] Setup
  (Utilities|FlowControl|Sequence
    (:then_0
      (if (Variables|Default|GetGameInProgress)
        (Utilities|FlowControl|Delay 1.0)
        (bind _output_get (Variables|Default|SetSeconds (+ (Variables|Default|GetSeconds) 1)))
        (if (> _output_get 59)
          (Variables|Default|SetMinutes (+ (Variables|Default|GetMinutes) 1))
          (Variables|Default|SetSeconds 0))))
    (:then_1
      (CallFunction|GazeCheck))))

(event Input|ActionEvents|InputActionOnRightClick
  (params (Key :type Key%20Structure :default "None"))
  ;[1 1 1] Gaze check
  (:Pressed
    (if (not (Variables|Default|GetDead))
      (if (.bBlockingHit (Collision|BreakHitResult (stale Custom|GazeCheck _outhit)))
        (Utilities|FlowControl|Sequence
          (:then_0
            (if (Utilities|DoesObjectImplementInterface (.HitActor (Collision|BreakHitResult (stale Custom|GazeCheck _outhit))) "/Game/Blueprints/Interface/BP_Door_Interface.BP_Door_Interface_C")
              (Class|BPDoorInterface|MoveDoor(Message) (.HitActor (Collision|BreakHitResult (stale Custom|GazeCheck _outhit))))))
          (:then_1
            (if (Utilities|DoesObjectImplementInterface (.HitActor (Collision|BreakHitResult (stale Custom|GazeCheck _outhit))) "/Game/Blueprints/Interface/BP_Interact_Interface.BP_Interact_Interface_C")
              (Class|BPLightInterface|LightInteract(Message) (.HitActor (Collision|BreakHitResult (stale Custom|GazeCheck _outhit))))
              (elif (not (Utilities|DoesObjectImplementInterface (.HitActor (Collision|BreakHitResult (stale Custom|GazeCheck _outhit))) "/Game/Blueprints/Interface/BP_Door_Interface.BP_Door_Interface_C"))
                (if (Utilities|DoesObjectImplementInterface (.HitActor (Collision|BreakHitResult (stale Custom|GazeCheck _outhit))) "/Game/Blueprints/Interface/BP_GameActivator_Interface.BP_GameActivator_Interface_C")
                  (Class|BPGameActivatorInterface|Activate(Message) (.HitActor (Collision|BreakHitResult (stale Custom|GazeCheck _outhit))))
                  (bind _asbp_game_activator (Utilities|Casting|CastToBP_GameActivator (.HitActor (Collision|BreakHitResult (stale Custom|GazeCheck _outhit)))))
                  (Variables|Default|SetGameInProgress (Variables|/Game/Blueprints/BP/BP_GameActivator.BP_GameActivator_C|GetGameInProgress _asbp_game_activator))
                  (else
                    (Transformation|Teleport (* (.Location (Collision|BreakHitResult (stale Custom|GazeCheck _outhit))) "1.000000,1.000000,1.000000") "0, 0, 0")))))))))))

(event Input|AxisEvents|InputAxismouseX
  (params (AxisValue :type Float%20%28single-precision%29))
  ;[1 1 1] Setup
  (Pawn|Input|AddControllerYawInput AxisValue))

(event Input|AxisEvents|InputAxismouseY
  (params (AxisValue :type Float%20%28single-precision%29))
  ;[1 1 1] Setup
  (Pawn|Input|AddControllerPitchInput AxisValue))

(fn ConstructionScript)