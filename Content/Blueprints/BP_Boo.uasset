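; BP_Boo is an actor that slowly homes in on the player's pawn unless its Frozen flag is set.
; Each Tick, it rotates to face player 0 and eases toward a point just along that pawn's forward vector with a slow, unswept VInterpTo.
; Nothing in this graph sets Frozen, and a WasRecentlyRendered check sits unconnected.
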(event EventBeginPlay)

(event Collision|EventActorBeginOverlap
  (params (OtherActor :type Actor%20Object%20Reference)))

(event EventTick
  (params (DeltaSeconds :type Float%20%28single-precision%29))
  (bind _returnvalue (Game|Player|GetPlayerPawn 0))
  (if (!= (Variables|Default|GetFrozen) true)
    (Transformation|SetActorRotation (Math|Rotator|FindLookatRotation (Transformation|GetActorLocation) (Transformation|GetActorLocation (Game|Player|GetPlayerPawn 0))))
    (Transformation|SetActorLocation (Math|Interpolation|VInterpTo (Transformation|GetActorLocation) (+ (Transformation|GetActorLocation _returnvalue) (Transformation|GetActorForwardVector _returnvalue)) DeltaSeconds 0.125) false false)))

(fn ConstructionScript)